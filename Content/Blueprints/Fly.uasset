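; Fly is an actor that drives procedural terrain generation around its own location.
; On BeginPlay it spawns a BP_ProceduralTerrain at the origin, sets its chunk size, surface shaping and material, then starts a looping timer.
; Each UpdateChunks tick converts the actor's XY position to chunk coordinates and calls GenerateFromOrigin for the surrounding area.
; A ToggleCollision call is present but never runs.
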(event Custom|UpdateChunks
  (bind _returnvalue (Transformation|GetActorLocation))
  (bind (_x _y _z) (Math|Vector|BreakVector _returnvalue))
  (Class|ProceduralTerrain|GeneratefromOrigin (Variables|Default|GetTerrainGeneratorInst) (Math|Float|Round (/ _x 3.2e+03)) (Math|Float|Round (/ _y 3.2e+03)) 0 10))

(event EventBeginPlay
  (Utilities|FlowControl|Sequence
    (:then_0
      (bind _returnvalue (Game|SpawnActorfromClass "/Game/Blueprints/BP_ProceduralTerrain.BP_ProceduralTerrain_C" (Math|Transform|MakeTransform "0, 0, 0") false 0))
      (Variables|Default|SetTerrainGeneratorInst _returnvalue))
    (:then_1
      (Variables|/Script/TerrainGenerator.ProceduralTerrain|SetChunkWidth (Variables|Default|GetTerrainGeneratorInst) 32)
      (Variables|/Script/TerrainGenerator.ProceduralTerrain|SetChunkLength (Variables|Default|GetTerrainGeneratorInst) 32)
      (Variables|/Script/TerrainGenerator.ProceduralTerrain|SetChunkHeight (Variables|Default|GetTerrainGeneratorInst) 32)
      (Variables|/Script/TerrainGenerator.ProceduralTerrain|SetGround (Variables|Default|GetTerrainGeneratorInst) 9)
      (Variables|/Script/TerrainGenerator.ProceduralTerrain|SetSurfaceCrossOverValue (Variables|Default|GetTerrainGeneratorInst) 0.0)
      (Variables|/Script/TerrainGenerator.ProceduralTerrain|SetgMaterial (Variables|Default|GetTerrainGeneratorInst) "/Game/Assets/Terrain/M_Landscape_SandRock_Inst.M_Landscape_SandRock_Inst")
      (Variables|/Script/TerrainGenerator.ProceduralTerrain|SetVerticalScaling (Variables|Default|GetTerrainGeneratorInst) 0.05)
      (Variables|/Script/TerrainGenerator.ProceduralTerrain|SetVerticalSmoothness (Variables|Default|GetTerrainGeneratorInst) 6.0)
      (Variables|/Script/TerrainGenerator.ProceduralTerrain|SetScale (Variables|Default|GetTerrainGeneratorInst) 1e+02)
      (Utilities|Time|SetTimerbyFunctionName 0 "UpdateChunks" 0.1 true))))

(fn ConstructionScript)